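; Bp_lisa is the Lisa character, whose audio cues follow game mode events.
; On BeginPlay it binds to two game mode dispatchers for the village entrance and the Lisa trigger.
; The entrance event adds a "psst" audio component; the trigger fades it out, then after a short delay plays the explanation cue at her location.
; The construction script disables PawnSensing updates.
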(event Custom|EdEntreeVillage_Event_0
  (bind _returnvalue (AddComponent|AddAudioComponent false))
  (Variables|Default|SetpsstRef _returnvalue))

(event Custom|EdTriggerLisa_Event_0
  (Audio|Components|Audio|FadeOut (Variables|Default|GetpsstRef) 0.5 0.0 "Linear" :!class /Script/Engine.AudioComponent)
  (Utilities|FlowControl|Delay 1.0)
  (Audio|PlaySoundatLocation "/Game/Sons/Lisa/Cue_explications.Cue_explications" (Transformation|GetActorLocation) "0, 0, 0" 1.0 1.0 0.0 0 0 0))

(event EventBeginPlay
  (bind _asgame_mode_ra (CallFunction|CastGmModeRa))
  (EventDispatchers|AssignEdEntreeVillage _asgame_mode_ra (delegate Custom|EdEntreeVillage_Event_0))
  (EventDispatchers|AssignEdTriggerLisa _asgame_mode_ra (delegate Custom|EdTriggerLisa_Event_0)))

(event Collision|EventActorBeginOverlap
  (params (OtherActor :type Actor%20Object%20Reference))
  (|CallParentFunction OtherActor) ; This node is disabled and will not be called.\nDrag off pins to build functionality.
)

(event EventTick
  (params (DeltaSeconds :type Float%20%28single-precision%29))
  (|CallParentFunction DeltaSeconds) ; This node is disabled and will not be called.\nDrag off pins to build functionality.
)

(fn ConstructionScript
  (|CallParentFunction)
  (Class|PawnSensingComponent|SetSensingUpdatesEnabled (Variables|Default|GetPawnSensing) false))