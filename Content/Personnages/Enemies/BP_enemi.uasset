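; Enemy character that wanders around its spawn point and chases the player on sight, destroying them when it reaches them.
; Patrol loops random reachable-point moves at walk speed with random pauses; PawnSensing triggers a faster chase once, gated by a DoOnce, and notifies the game mode.
; Game mode safe-zone events disable sensing and resume patrol, or re-enable sensing and reset the chase gate.
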(event OnSeePawn(PawnSensing)
  (params (Pawn :type Pawn%20Object%20Reference))
  ;[1 1 1] on see pawn
  (if (== Pawn (Game|GetPlayerCharacter 0))
    (Utilities|FlowControl|DoOnce false
      (:Completed
        (CallFunction|Poursuite)
        (Default|CallEdPoursuite (CallFunction|CastGmModeRa))))))

(event Custom|Poursuite
  (bind _returnvalue (Game|GetPlayerCharacter 0))
  ;[1 1 1] Poursuite
  (if (Utilities|Time|IsValidTimerHandle (Variables|Default|GetrondeTimerRef))
    (Utilities|Time|ClearandInvalidateTimerbyHandle (Variables|Default|GetrondeTimerRef)))
  (Variables|/Script/Engine.CharacterMovementComponent|SetMaxWalkSpeed (Variables|Character|GetCharacterMovement) 3e+02)
  (AI|AIMoveTo self "0, 0, 0" (Game|GetPlayerCharacter 0) 2e+01 false
    (:OnSuccess
      (Utilities|IsValid _returnvalue
        (:Is%20Valid
          (Actor|DestroyActor _returnvalue))))))

(event Custom|ronde
  ;[1 1 1] Ronde
  (Variables|/Script/Engine.CharacterMovementComponent|SetMaxWalkSpeed (Variables|Character|GetCharacterMovement) 1.5e+02)
  (AI|AIMoveTo self (.RandomLocation (AI|Navigation|GetRandomReachablePointinRadius (Variables|Default|GetlocationDepart) 1e+03 0 0)) 0 2e+01 false
    (:OnSuccess
      (bind _returnvalue (Utilities|Time|SetTimerbyFunctionName 0 "ronde" (Math|Random|RandomFloatinRange 0.5 8.0)))
      (Variables|Default|SetrondeTimerRef _returnvalue))))

(event Custom|resetPoursuit
  ;[1 1 1] on see pawn
  (Utilities|FlowControl|DoOnce false) ; enters at Reset
)

(event Custom|EdSafeZoneOn_Event_0
  (Variables|/Script/AIModule.PawnSensingComponent|SetbSeePawns (Variables|Default|GetPawnSensing) false)
  (CallFunction|Ronde))

(event Custom|EdSafeZoneOff_Event_0
  (Variables|/Script/AIModule.PawnSensingComponent|SetbSeePawns (Variables|Default|GetPawnSensing) true)
  (CallFunction|ResetPoursuit))

(event EventBeginPlay
  (bind _asgame_mode_ra (CallFunction|CastGmModeRa))
  (EventDispatchers|AssignEdSafeZoneon _asgame_mode_ra (delegate Custom|EdSafeZoneOn_Event_0))
  (EventDispatchers|AssignEdSafeZoneOff _asgame_mode_ra (delegate Custom|EdSafeZoneOff_Event_0))
  (Variables|Default|SetlocationDepart (Transformation|GetActorLocation))
  (CallFunction|Ronde))

(event Collision|EventActorBeginOverlap
  (params (OtherActor :type Actor%20Object%20Reference)))

(event EventTick
  (params (DeltaSeconds :type Float%20%28single-precision%29)))

(fn ConstructionScript)