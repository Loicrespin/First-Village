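; Pistol weapon Blueprint that handles firing, reloading and ammo pickup, tracking a magazine and a reserve.
; On BeginPlay it binds to the game mode's fire, reload and pickup event dispatchers and caches its AnimPistol AnimBP.
; Firing flags the animation, spends a round and applies random damage to the actor in the supplied hit result.
; Reload moves rounds from the reserve, and every ammo change updates the player controller's main UI.
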(event Custom|EdTirer_Event_0
  (params (hit :type Hit%20Result%20Structure))
  ;[1 1 1] Ed Tirer
  (CallFunction|Shoot hit))

(event Custom|EdRecharger_Event_0
  ;[1 1 1] Ed reload
  (CallFunction|Recharger))

(event Custom|EdPickupAmmo_Event_0
  (params (nbBalles :type Integer))
  ;[1 1 1] Ed Pickup Ammo
  (CallFunction|MajMunitions nbBalles))

(event EventBeginPlay
  (Variables|Default|SetGmRef (CallFunction|CastGmModeRa))
  (Variables|Default|SetpcRef (CallFunction|CastPcRa))
  (Utilities|FlowControl|Sequence
    (:then_0
      ;[1 1 1] Ed Tirer
      (EventDispatchers|AssignEdTirer (Variables|Default|GetGmRef) (delegate Custom|EdTirer_Event_0)))
    (:then_1
      ;[1 1 1] AnimBp Pistolet
      (bind _asanim_pistol (Utilities|Casting|CastToAnimPistol (Components|SkeletalMesh|GetAnimInstance (Variables|Default|GetSkeletalMesh))))
      (Variables|Default|SetanimRef _asanim_pistol))
    (:then_2
      ;[1 1 1] Ed reload
      (EventDispatchers|AssignEdRecharger (Variables|Default|GetGmRef) (delegate Custom|EdRecharger_Event_0)))
    (:then_3
      ;[1 1 1] Ed Pickup Ammo
      (EventDispatchers|AssignEdPickupAmmo (Variables|Default|GetGmRef) (delegate Custom|EdPickupAmmo_Event_0)))))

(fn ConstructionScript)

(fn Shoot
  (params (hit :type Hit%20Result%20Structure))
  (if (> (Variables|Default|Getchargeur) 0)
    (Variables|/Game/Imports/MilitaryWeapDark/Weapons/AnimPistol.AnimPistol_C|Setshooting (Variables|Default|GetanimRef) true)
    (Math|Integer|DecrementInt (Variables|Default|Getchargeur)
      (:%20%20
        (Game|Damage|ApplyDamage (.HitActor (Collision|BreakHitResult hit)) (Math|Random|RandomFloatinRange 5e+01 1.5e+02) (Game|GetPlayerController 0) (Game|GetPlayerCharacter 0))
        (Default|AfficherMunitions (Variables|/Game/System/PlayerControllerRA.PlayerControllerRA_C|GetUi%20MainRef (Variables|Default|GetpcRef)) true (Variables|Default|Getchargeur))))))

(fn Recharger
  (if (> (Variables|Default|Getmunitions) 0)
    (LocalVariables|SetnbrReload (Math|Integer|Clamp(Integer) (- (Variables|Default|GetchargeurMax) (Variables|Default|Getchargeur)) 0 (Variables|Default|Getmunitions)))
    (Variables|Default|Setchargeur (+ (Variables|Default|Getchargeur) (LocalVariables|GetnbrReload)))
    (Variables|Default|Setmunitions (- (Variables|Default|Getmunitions) (LocalVariables|GetnbrReload)))
    (Default|AfficherMunitions (Variables|/Game/System/PlayerControllerRA.PlayerControllerRA_C|GetUi%20MainRef (Variables|Default|GetpcRef)) true (Variables|Default|Getchargeur))
    (Default|AfficherMunitions (Variables|/Game/System/PlayerControllerRA.PlayerControllerRA_C|GetUi%20MainRef (Variables|Default|GetpcRef)) false (Variables|Default|Getmunitions))
    (else
      (Development|PrintString "A sec"))))

(fn MajMunitions
  (params (nbrBalles :type Integer))
  (bind _output_get (Variables|Default|Setmunitions (+ nbrBalles (Variables|Default|Getmunitions))))
  (Default|AfficherMunitions (Variables|/Game/System/PlayerControllerRA.PlayerControllerRA_C|GetUi%20MainRef (Variables|Default|GetpcRef)) false _output_get))