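; Camera actor that plays a short timed view cut when the game mode's EdTriggerLisa event fires.
; On BeginPlay it gets the game mode through CastGmModeRa and binds to that trigger.
; When triggered, it blends the player's view to itself and disables character input.
; After a delay it blends back, restores input and calls EdTriggerLisaOut on the game mode as the return blend starts.
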(event Custom|EdTriggerLisa_Event_0
  (bind _returnvalue (Game|GetPlayerController 0))
  (bind _returnvalue_2 (Game|GetPlayerController 0))
  (Game|Player|SetViewTargetwithBlend _returnvalue_2 self 2.0 "VTBlend_Linear" 0.0 false)
  (Input|DisableInput (Game|GetPlayerCharacter 0) _returnvalue_2)
  (Utilities|FlowControl|Delay 5.0)
  (Game|Player|SetViewTargetwithBlend _returnvalue (Game|GetPlayerCharacter 0) 2.0 "VTBlend_Linear" 0.0 false)
  (Input|EnableInput (Game|GetPlayerCharacter 0) _returnvalue)
  (Default|CallEdTriggerLisaOut (Variables|Default|GetGmRef)))

(event EventBeginPlay
  (Variables|Default|SetGmRef (CallFunction|CastGmModeRa))
  (EventDispatchers|AssignEdTriggerLisa (Variables|Default|GetGmRef) (delegate Custom|EdTriggerLisa_Event_0)))

(fn ConstructionScript)