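; BP_caisse is an interactable crate that acts as a collectible objective, repairing the car, arming the hero and triggering wave management.
; On IInteragir, it registers itself as collected with the game mode cached at BeginPlay and refreshes the mission UI.
; It then flags the first Bp_voiture found as repaired and makes the player's BP_heros equip a weapon.
; After a short delay, it calls GestionVagues on the game mode.
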(event EventBeginPlay
  (|CallParentFunction)
  (Variables|Default|SetgmRef (CallFunction|CastGmModeRa)))

(event Collision|EventActorBeginOverlap
  (params (OtherActor :type Actor%20Object%20Reference))
  (|CallParentFunction OtherActor) ; This node is disabled and will not be called.\nDrag off pins to build functionality.
)

(event EventTick
  (params (DeltaSeconds :type Float%20%28single-precision%29))
  (|CallParentFunction DeltaSeconds) ; This node is disabled and will not be called.\nDrag off pins to build functionality.
)

(event EventIInteragir
  (Default|MajObjetCollecte (Variables|Default|GetgmRef) self)
  (Default|AfficherMissions (Variables|/Game/System/PlayerControllerRA.PlayerControllerRA_C|GetUi%20MainRef (CallFunction|CastPcRa)))
  (bind _outactors (Actor|GetAllActorsOfClass "/Game/Blueprints/Bp_voiture.Bp_voiture_C"))
  (Variables|/Game/Blueprints/Bp_voiture.Bp_voiture_C|Setreparee (Utilities|Array|Get(acopy) _outactors) true)
  (bind _asbp_heros (Utilities|Casting|CastToBP_heros (Game|GetPlayerCharacter 0)))
  (Default|EquiperArme _asbp_heros)
  (Utilities|FlowControl|Delay 5.0)
  (Default|GestionVagues (Variables|Default|GetgmRef)))

(fn ConstructionScript
  (|CallParentFunction))