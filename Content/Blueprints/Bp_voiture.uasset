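; Interactable car actor that responds to the IInteragir event according to whether it has been repaired.
; When repaired, it only prints a debug string.
; When not repaired, it adds an audio component on first use and caches it in CueVoitureRef, then replays that cue on later interactions only if it is not already playing.
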(event EventBeginPlay
  (|CallParentFunction) ; This node is disabled and will not be called.\nDrag off pins to build functionality.
)

(event Collision|EventActorBeginOverlap
  (params (OtherActor :type Actor%20Object%20Reference))
  (|CallParentFunction OtherActor) ; This node is disabled and will not be called.\nDrag off pins to build functionality.
)

(event EventTick
  (params (DeltaSeconds :type Float%20%28single-precision%29))
  (|CallParentFunction DeltaSeconds) ; This node is disabled and will not be called.\nDrag off pins to build functionality.
)

(event EventIInteragir
  (if (Variables|Default|Getreparee)
    (Development|PrintString "reparee")
    (else
      ;[1 1 1] Voiture non reparee
      (Utilities|IsValid (Variables|Default|GetcueVoitureRef)
        (:Is%20Valid
          (if (not (Audio|Components|Audio|IsPlaying (Variables|Default|GetcueVoitureRef)))
            (Audio|Components|Audio|Play (Variables|Default|GetcueVoitureRef) 0.0)))
        (:Is%20Not%20Valid
          (bind _returnvalue (AddComponent|AddAudioComponent false))
          (Variables|Default|SetcueVoitureRef _returnvalue))))))

(fn ConstructionScript
  (|CallParentFunction))