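; Safe zone actor that signals the game mode when the player character enters or leaves its box while it is active.
; Box overlaps trigger the game mode's SafeZoneOn and SafeZoneOff dispatchers.
; It also listens to SafeZoneOff itself, so each such broadcast hides the cube and deactivates the zone for an inactive period before restoring both.
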(event OnComponentBeginOverlap(Box)
  (params (OverlappedComponent :type Primitive%20Component%20Object%20Reference) (OtherActor :type Actor%20Object%20Reference) (OtherComp :type Primitive%20Component%20Object%20Reference) (OtherBodyIndex :type Integer) (bFromSweep :type Boolean) (SweepResult :type Hit%20Result%20Structure%20%28by%20ref%29))
  ;[1 1 1] Quand on entre dans la Safezone
  (if (and (== OtherActor (Game|GetPlayerCharacter 0)) (Variables|Default|Getactive))
    (Default|CallEdSafeZoneon (CallFunction|CastGmModeRa))))

(event OnComponentEndOverlap(Box)
  (params (OverlappedComponent :type Primitive%20Component%20Object%20Reference) (OtherActor :type Actor%20Object%20Reference) (OtherComp :type Primitive%20Component%20Object%20Reference) (OtherBodyIndex :type Integer))
  ;[1 1 1] Quand on sort de la Safezone
  (if (and (== OtherActor (Game|GetPlayerCharacter 0)) (Variables|Default|Getactive))
    (Default|CallEdSafeZoneOff (CallFunction|CastGmModeRa))))

(event Custom|EdSafeZoneOff_Event_0
  (CallFunction|GestionActivation false)
  (Utilities|FlowControl|Delay (Variables|Default|GetperiodeInactive))
  (CallFunction|GestionActivation true))

(event EventBeginPlay
  (EventDispatchers|AssignEdSafeZoneOff (CallFunction|CastGmModeRa) (delegate Custom|EdSafeZoneOff_Event_0)))

(event Collision|EventActorBeginOverlap
  (params (OtherActor :type Actor%20Object%20Reference)))

(event EventTick
  (params (DeltaSeconds :type Float%20%28single-precision%29)))

(fn ConstructionScript)

(fn GestionActivation
  (params (activer :type Boolean))
  (if activer
    (Development|SetHiddeninGame (Variables|Default|GetCube) false false)
    (Variables|Default|Setactive true)
    (else
      (Development|SetHiddeninGame (Variables|Default|GetCube) true false)
      (Variables|Default|Setactive false))))