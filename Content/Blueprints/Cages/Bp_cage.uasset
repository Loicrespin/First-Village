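; Cage actor whose Rope physics constraint is driven to sway back and forth as if in wind.
; Every tick, WindRope sets the constraint's angular velocity target on X and Y to a game-time sine wave, using SpeedUpTime for frequency and Magnitude for strength.
; Its inactive branch zeroes both variables, but Tick always passes true.
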(event EventBeginPlay)

(event Collision|EventActorBeginOverlap
  (params (OtherActor :type Actor%20Object%20Reference)))

(event EventTick
  (params (DeltaSeconds :type Float%20%28single-precision%29))
  (CallFunction|WindRope true))

(fn ConstructionScript)

(fn WindRope
  (params (active :type Boolean))
  (if active
    (Class|PhysicsConstraintComponent|SetAngularVelocityTarget (Variables|Default|GetRope) (Math|Vector|MakeVector (* (Math|Trig|Sin(Radians) (* (Utilities|Time|GetGameTimeinSeconds) (Variables|Default|GetspeedUpTime))) (Variables|Default|Getmagnitude)) (* (Math|Trig|Sin(Radians) (* (Utilities|Time|GetGameTimeinSeconds) (Variables|Default|GetspeedUpTime))) (Variables|Default|Getmagnitude)) 0.0))
    (else
      (Variables|Default|SetspeedUpTime 0.0)
      (Variables|Default|Setmagnitude 0.0))))