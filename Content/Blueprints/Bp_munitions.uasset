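; Ammo pickup actor that gives the player a random number of bullets when interacted with.
; The construction script rolls the bullet count between a small minimum and maximum.
; On the IInteragir interface event, it plays a pickup sound, passes the count to the GmModeRa game mode through CallEdPickupAmmo, then destroys itself.
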(event EventBeginPlay
  (|CallParentFunction) ; This node is disabled and will not be called.\nDrag off pins to build functionality.
)

(event Collision|EventActorBeginOverlap
  (params (OtherActor :type Actor%20Object%20Reference))
  (|CallParentFunction OtherActor) ; This node is disabled and will not be called.\nDrag off pins to build functionality.
)

(event EventTick
  (params (DeltaSeconds :type Float%20%28single-precision%29))
  (|CallParentFunction DeltaSeconds) ; This node is disabled and will not be called.\nDrag off pins to build functionality.
)

(event EventIInteragir
  (Audio|PlaySound2D "/Game/MilitaryWeapDark/Sound/Pistol/Pistol_AmmoPickup_Cue.Pistol_AmmoPickup_Cue" 1.0 1.0 0.0 0 0)
  (Default|CallEdPickupAmmo (CallFunction|CastGmModeRa) (Variables|Default|GetnbBalles))
  (Actor|DestroyActor))

(fn ConstructionScript
  (|CallParentFunction)
  (Variables|Default|SetnbBalles (Math|Random|RandomIntegerinRange 2 10)))